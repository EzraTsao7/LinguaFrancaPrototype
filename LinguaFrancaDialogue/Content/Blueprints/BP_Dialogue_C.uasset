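; Dialogue component that feeds lines and speaker names to the player character one at a time.
; Each StartSpeaking call either interrupts the line being spoken or advances to the next, passing it through player-character messages.
; Per-line arrays supply text speed and auto-advance, with a nonzero TextSpeed overriding speed and ManualAdvance disabling auto-advance.
; After the last line it resets, signals completion and optionally destroys itself.
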(event Custom|StartSpeaking
  (bind _returnvalue (Game|GetPlayerCharacter 0))
  (bind _dialogue (Variables|Default|GetDialogue))
  (bind _textspeed (Variables|Default|GetTextSpeed))
  (bind _manualadvance (Variables|Default|GetManualAdvance))
  (bind _check (Class|BPIDialogue|CurrentlySpeaking(Message) _returnvalue))
  (if _check
    (if (Variables|Default|GetManualAdvance)
      (Class|BPIDialogue|InteruptSpeaking(Message) _returnvalue (Utilities|Array|Get(acopy) _dialogue (Variables|Default|GetCurrentLine)) false (Utilities|Array|Get(acopy) (Variables|Default|GetSpeaker) (Variables|Default|GetCurrentLine)))
      (else
        (Class|BPIDialogue|InteruptSpeaking(Message) _returnvalue (Utilities|Array|Get(acopy) _dialogue (Variables|Default|GetCurrentLine)) (Utilities|Array|Get(acopy) (Variables|Default|GetAdvanceVarying) (Variables|Default|GetCurrentLine)) (Utilities|Array|Get(acopy) (Variables|Default|GetSpeaker) (Variables|Default|GetCurrentLine)))))
    (elif (>= (Variables|Default|GetCurrentLine) (- (Utilities|Array|Length _dialogue) 1))
      (Variables|Default|SetCurrentLine -1)
      (Class|BPIDialogue|FinishedSpeaking(Message) _returnvalue)
      (if (Variables|Default|GetSelfDestruct)
        (Components|DestroyComponent))
      (else
        (Math|Integer|IncrementInt (Variables|Default|GetCurrentLine)
          (:%20%20
            (if (== (Variables|Default|GetTextSpeed) 0.0)
              (if _manualadvance
                (Class|BPIDialogue|Speaking(Message) _returnvalue (Utilities|Array|Get(acopy) _dialogue (Variables|Default|GetCurrentLine)) (Utilities|Array|Get(acopy) (Variables|Default|GetTextSpeedVarying) (Variables|Default|GetCurrentLine)) false (Utilities|Array|Get(acopy) (Variables|Default|GetSpeaker) (Variables|Default|GetCurrentLine)))
                (else
                  (Class|BPIDialogue|Speaking(Message) _returnvalue (Utilities|Array|Get(acopy) _dialogue (Variables|Default|GetCurrentLine)) (Utilities|Array|Get(acopy) (Variables|Default|GetTextSpeedVarying) (Variables|Default|GetCurrentLine)) (Utilities|Array|Get(acopy) (Variables|Default|GetAdvanceVarying) (Variables|Default|GetCurrentLine)) (Utilities|Array|Get(acopy) (Variables|Default|GetSpeaker) (Variables|Default|GetCurrentLine)))))
              (elif _manualadvance
                (Class|BPIDialogue|Speaking(Message) _returnvalue (Utilities|Array|Get(acopy) _dialogue (Variables|Default|GetCurrentLine)) _textspeed false (Utilities|Array|Get(acopy) (Variables|Default|GetSpeaker) (Variables|Default|GetCurrentLine)))
                (else
                  ;[1 1 1] Auto Advance, Consistent Speed
                  (Class|BPIDialogue|Speaking(Message) _returnvalue (Utilities|Array|Get(acopy) _dialogue (Variables|Default|GetCurrentLine)) _textspeed (Utilities|Array|Get(acopy) (Variables|Default|GetAdvanceVarying) (Variables|Default|GetCurrentLine)) (Utilities|Array|Get(acopy) (Variables|Default|GetSpeaker) (Variables|Default|GetCurrentLine))))))))))))